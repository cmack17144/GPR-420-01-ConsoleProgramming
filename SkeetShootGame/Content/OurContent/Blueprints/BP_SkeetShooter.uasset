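; Skeet launcher actor that repeatedly spawns flattened BP_Skeet targets at its Arrow component.
; BeginPlay calls StartShooting directly and through a one-second timer, which enables ShouldShoot and starts a looping ShootSkeet timer.
; Each shot pushes the skeet along the Arrow's forward vector with slight random variation, using mass-independent force.
; ShootSkeet clears the looping timer when it finds ShouldShoot false.
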(event Custom|StartShooting
  (bind _output_get (Variables|Default|SetShouldShoot true))
  (bind _returnvalue (Utilities|Time|SetTimerbyEvent (delegate Custom|ShootSkeet) (Variables|Default|GetShootInterval) true))
  (CallFunction|ShootSkeet))

(event Custom|ShootSkeet
  (bind _arrow (Variables|Default|GetArrow))
  (bind _returnvalue (Transformation|GetWorldTransform _arrow))
  (bind (_location _rotation) (Math|Transform|BreakTransform _returnvalue))
  (if (stale Custom|StartShooting _output_get) ; Should stop if game stops
    (bind _returnvalue_2 (Game|SpawnActorfromClass "/Game/OurContent/Blueprints/BP_Skeet.BP_Skeet_C" (Math|Transform|MakeTransform _location _rotation "1.000000,1.000000,0.150000") "AlwaysSpawn" 0 0))
    (Physics|AddForce (Variables|/Game/OurContent/Blueprints/BP_Skeet.BP_Skeet_C|GetStaticMesh _returnvalue_2) (+ (* (Math|Vector|GetForwardVector _arrow) (Variables|Default|GetShootForce)) (* (Math|Random|RandomUnitVector) 5e+01)) "None" true)
    (else
      (Utilities|Time|ClearandInvalidateTimerbyHandle (stale Custom|StartShooting _returnvalue)))))

(event EventBeginPlay
  (Variables|Default|SetShouldShoot false) ; Gets set to tru when game starts
  (Utilities|Time|SetTimerbyEvent (delegate Custom|StartShooting) 1.0)
  (CallFunction|StartShooting))

(fn ConstructionScript)