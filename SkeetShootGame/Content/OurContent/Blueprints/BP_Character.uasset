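; Player character that tracks a named score and records it in a saved local leaderboard.
; BeginPlay shows a name-entry widget and disables mouse look; DrawScore adds the score HUD and re-enables it.
; AddScore increments the score, and the Decimal key saves it to an LB_Save slot, keeping each name's best, and feeds the leaderboard widget.
; Also handles basic movement and look input.
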(event Custom|DrawLeaderBoard
  (bind _data_lbsave (Variables|Default|GetData%20LBSave))
  ;[1 1 1] Widgets - LeaderBoard
  (Widget|RemovefromParent (Variables|Default|GetScoreWidget))
  (bind _returnvalue (UserInterface|CreateWidget "/Game/OurContent/Blueprints/LB_LeaderBoard.LB_LeaderBoard_C"))
  (Class|UserWidget|SetAlignmentinViewport _returnvalue "(X=0.500000,Y=0.500000)")
  (Class|UserWidget|SetAnchorsinViewport _returnvalue (Utilities|Struct|MakeAnchors "(X=0.500000,Y=0.500000)" "(X=0.500000,Y=0.500000)"))
  (Class|UserWidget|SetPositioninViewport _returnvalue (/ (Viewport|GetViewportSize) 2.0) true)
  (Class|UserWidget|SetDesiredSizeinViewport _returnvalue "(X=500.000000,Y=800.000000)")
  (UserInterface|Viewport|AddtoViewport _returnvalue 0)
  (Default|AddData _returnvalue (Variables|/Game/OurContent/Blueprints/LB_Save.LB_Save_C|GetUserNames _data_lbsave) (Variables|/Game/OurContent/Blueprints/LB_Save.LB_Save_C|GetUserScores _data_lbsave)))

(event Custom|Name%20Prompt
  ;[1 1 1] Widgets - Name Prompt
  (bind _returnvalue (UserInterface|CreateWidget "/Game/OurContent/Blueprints/LB_CreateName.LB_CreateName_C"))
  (Class|UserWidget|SetAlignmentinViewport _returnvalue "(X=0.500000,Y=0.500000)")
  (Class|UserWidget|SetAnchorsinViewport _returnvalue (Utilities|Struct|MakeAnchors "(X=0.500000,Y=0.500000)" "(X=0.500000,Y=0.500000)"))
  (Class|UserWidget|SetPositioninViewport _returnvalue (/ (Viewport|GetViewportSize) 2.0) true)
  (Class|UserWidget|SetDesiredSizeinViewport _returnvalue "(X=500.000000,Y=300.000000)")
  (UserInterface|Viewport|AddtoViewport _returnvalue 0)
  (Variables|Default|SetNameWidget _returnvalue)
  (Variables|Default|SetControlsEnabled false)
  (Variables|/Script/Engine.PlayerController|SetbShowMouseCursor (Game|GetPlayerController 0) true))

(event Custom|Draw%20Score
  ;[1 1 1] Widgets - Score
  (bind _returnvalue (UserInterface|CreateWidget "/Game/OurContent/Blueprints/LB_Score.LB_Score_C"))
  (Class|UserWidget|SetAlignmentinViewport _returnvalue "(X=0.500000,Y=0.000000)")
  (Class|UserWidget|SetAnchorsinViewport _returnvalue (Utilities|Struct|MakeAnchors "(X=0.500000,Y=0.000000)" "(X=0.500000,Y=0.000000)"))
  (Class|UserWidget|SetPositioninViewport _returnvalue (Math|Vector2D|MakeVector2D (/ (.X (Math|Vector2D|BreakVector2D (Viewport|GetViewportSize))) 2.0) 25.0) true)
  (Class|UserWidget|SetDesiredSizeinViewport _returnvalue "(X=400.000000,Y=100.000000)")
  (UserInterface|Viewport|AddtoViewport _returnvalue 0)
  (Development|PrintString (Variables|Default|GetUserName))
  (Variables|Default|SetControlsEnabled true)
  (Variables|/Script/Engine.PlayerController|SetbShowMouseCursor (Game|GetPlayerController 0) false)
  (Variables|Default|SetScoreWidget _returnvalue))

(event EventBeginPlay
  (CallFunction|NamePrompt))

(event Input|AxisEvents|InputAxisMoveForward
  (params (AxisValue :type Float%20%28single-precision%29))
  ;[1 1 1] Basic Movement Controls
  (Pawn|Input|AddMovementInput (Math|Vector|GetForwardVector (Pawn|GetControlRotation :!class /Script/Engine.Pawn)) AxisValue false))

(event Input|AxisEvents|InputAxisMoveRight
  (params (AxisValue :type Float%20%28single-precision%29))
  ;[1 1 1] Basic Movement Controls
  (Pawn|Input|AddMovementInput (Math|Vector|GetRightVector (Pawn|GetControlRotation :!class /Script/Engine.Pawn)) AxisValue false))

(event Input|AxisEvents|InputAxisLookRight
  (params (AxisValue :type Float%20%28single-precision%29))
  ;[1 1 1] Basic Movement Controls
  (Pawn|Input|AddControllerYawInput AxisValue))

(event Input|AxisEvents|InputAxisLookUp
  (params (AxisValue :type Float%20%28single-precision%29))
  ;[1 1 1] Basic Movement Controls
  (Pawn|Input|AddControllerPitchInput AxisValue))

(event Input|MouseEvents|MouseY
  (params (AxisValue :type Float%20%28single-precision%29))
  ;[1 1 1] Control Mouse Input Bool
  (if (Variables|Default|GetControlsEnabled)
    (Pawn|Input|AddControllerPitchInput (* AxisValue -1.0))))

(event Input|MouseEvents|MouseX
  (params (AxisValue :type Float%20%28single-precision%29))
  ;[1 1 1] Control Mouse Input Bool
  (if (Variables|Default|GetControlsEnabled)
    (Pawn|Input|AddControllerYawInput AxisValue)))

(event Input|KeyboardEvents|Decimal
  (params (Key :type Key%20Structure :default "None"))
  (bind _lb_slotname (Variables|Default|GetLB_SlotName))
  (bind _userscore (Variables|Default|GetUserScore))
  ;[1 1 1] Save
  (:Pressed
    (bind _returnvalue (SaveGame|DoesSaveGameExist (Variables|Default|GetLB_SlotName)))
    (if _returnvalue
      (bind _returnvalue_2 (SaveGame|LoadGamefromSlot (Variables|Default|GetLB_SlotName)))
      (bind _aslb_save (Utilities|Casting|CastToLB_Save _returnvalue_2))
      (bind _output_get (Variables|Default|SetData%20LBSave _aslb_save))
      ;[1 1 1] Checks to see if name already exists and updates score if true
      (if (Utilities|Array|ContainsItem (Variables|/Game/OurContent/Blueprints/LB_Save.LB_Save_C|GetUserNames _output_get) (Variables|Default|GetUserName))
        (Math|Integer|CompareInt (Utilities|Array|Get(acopy) (Variables|/Game/OurContent/Blueprints/LB_Save.LB_Save_C|GetUserScores _output_get) (Utilities|Array|FindItem (Variables|/Game/OurContent/Blueprints/LB_Save.LB_Save_C|GetUserNames _output_get) (Variables|Default|GetUserName))) _userscore
          (:>
            _)
          (:==
            _)
          (:<
            (Utilities|Array|SetArrayElem (Variables|/Game/OurContent/Blueprints/LB_Save.LB_Save_C|GetUserScores _output_get) (Utilities|Array|FindItem (Variables|/Game/OurContent/Blueprints/LB_Save.LB_Save_C|GetUserNames _output_get) (Variables|Default|GetUserName)) _userscore)
            (SaveGame|SaveGametoSlot (Variables|Default|GetData%20LBSave) _lb_slotname :!label _label)))
        (else
          (Utilities|Array|Add (Variables|/Game/OurContent/Blueprints/LB_Save.LB_Save_C|GetUserNames _output_get) (Variables|Default|GetUserName))
          (Utilities|Array|Add (Variables|/Game/OurContent/Blueprints/LB_Save.LB_Save_C|GetUserScores _output_get) (Variables|Default|GetUserScore))
          (goto _label)))
      (else
        (bind _returnvalue_3 (SaveGame|CreateSaveGameObject "/Game/OurContent/Blueprints/LB_Save.LB_Save_C"))
        (bind _aslb_save_2 (Utilities|Casting|CastToLB_Save _returnvalue_3))
        (bind _output_get_2 (Variables|Default|SetData%20LBSave _aslb_save_2))
        (Utilities|Array|Add (Variables|/Game/OurContent/Blueprints/LB_Save.LB_Save_C|GetUserNames _output_get_2) (Variables|Default|GetUserName))
        (Utilities|Array|Add (Variables|/Game/OurContent/Blueprints/LB_Save.LB_Save_C|GetUserScores _output_get_2) (Variables|Default|GetUserScore))
        (SaveGame|SaveGametoSlot (Variables|Default|GetData%20LBSave) _lb_slotname)))
    (CallFunction|DrawLeaderBoard)))

(fn ConstructionScript)

(fn AddScore
  (Variables|Default|SetUserScore (+ (Variables|Default|GetUserScore) 1)))