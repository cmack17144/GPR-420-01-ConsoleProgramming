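; BP_GameMode is the game mode that runs a timed round and tells the player character when to prompt for a name and save.
; On BeginPlay it calls NamePrompt on BP_Character if the level is "mainlevel".
; StartTimer resets the time left to GameTime and starts the countdown in Tick.
; When time runs out, it calls SaveCall on the character and clears the started flag.
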(event Custom|StartTimer
  (Variables|Default|SetTimeLeft (Variables|Default|GetGameTime))
  (Variables|Default|SetGameStarted true))

(event EventTick
  (params (DeltaSeconds :type Float%20%28single-precision%29))
  ;[1 1 1] If game started then decrement time left
  (if (Variables|Default|GetGameStarted)
    (bind _output_get (Variables|Default|SetTimeLeft (- (Variables|Default|GetTimeLeft) DeltaSeconds)))
    ;[1 1 1] End game if time left <= 0
    (if (<= _output_get 0.0)
      (bind _asbp_character (Utilities|Casting|CastToBP_Character (Game|Player|GetPlayerPawn 0)))
      (Default|SaveCall _asbp_character)
      (Variables|Default|SetGameStarted false))))

(event EventBeginPlay
  (bind _returnvalue (Game|GetCurrentLevelName true))
  (if (Utilities|Enum|Equal(Enum) _returnvalue "mainlevel")
    (bind _asbp_character (Utilities|Casting|CastToBP_Character (Game|Player|GetPlayerPawn 0)))
    (Default|NamePrompt _asbp_character)))

(fn ConstructionScript)