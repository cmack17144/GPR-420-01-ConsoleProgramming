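; BP_Weapon is a weapon actor that fires projectiles toward where the player's camera is looking.
; On BeginPlay it stores its parent actor as a BP_Character to access the player camera.
; Fire input line-traces from the muzzle to a distant point along the camera's forward vector.
; It spawns BP_Projectile at the muzzle, rotated toward the trace's end point rather than any impact point.
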(event EventBeginPlay
  ;[1 1 1] On begin get reference to the controller in parent
  (bind _asbp_character (Utilities|Casting|CastToBP_Character (Actor|GetParentActor))
    (:then
      (Variables|Default|SetController _asbp_character))
    (:CastFailed
      (Development|PrintString "Broke"))))

(event Input|ActionEvents|InputActionFire
  (params (Key :type Key%20Structure :default "None"))
  (bind _controller (Variables|Default|GetController))
  (bind _muzzle (Variables|Default|GetMuzzle))
  (bind _returnvalue (Transformation|GetWorldLocation _muzzle))
  (bind _playercamera (Variables|/Game/OurContent/Blueprints/BP_Character.BP_Character_C|GetPlayerCamera _controller))
  (:Pressed
    (bind _outhit (Collision|LineTraceByChannel _returnvalue (+ (Transformation|GetWorldLocation _playercamera) (* (Math|Vector|GetForwardVector _playercamera) 5e+03)) "TraceTypeQuery1" false 0 "None"))
    (Game|SpawnActorfromClass "/Game/OurContent/Blueprints/BP_Projectile.BP_Projectile_C" (Math|Transform|MakeTransform _returnvalue (Math|Rotator|FindLookatRotation _returnvalue (.TraceEnd (Collision|BreakHitResult _outhit)))) "Undefined" 0 0)))

(fn ConstructionScript)